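; Moving carpet pad that launches BP_ThirdPersonCharacter along positive or negative world X when it enters the box.
; The Acceleration timeline, re-played on Tick, sets the launch direction by whether its value exceeds the midpoint.
; Its updates also blend the plane's color, feed the material's acceleration value and play a Scale timeline that resizes the actor along X.
; The construction script sets up the M_Accel dynamic material's UV scale, arrow and parallax speeds, and colors.
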(event OnComponentBeginOverlap(Box)
  (params (OverlappedComponent :type Primitive%20Component%20Object%20Reference) (OtherActor :type Actor%20Object%20Reference) (OtherComp :type Primitive%20Component%20Object%20Reference) (OtherBodyIndex :type Integer) (bFromSweep :type Boolean) (SweepResult :type Hit%20Result%20Structure%20%28by%20ref%29))
  (bind _asbp_third_person_character (Utilities|Casting|CastToBP_ThirdPersonCharacter OtherActor))
  (CallFunction|AccelPlayer (> (stale EventBeginPlay _accel) (Variables|Default|GetaccelMiddle)) _asbp_third_person_character))

(event EventBeginPlay
  (bind _accel (Timeline|Acceleration Play)
    (:Update
      (bind _scale (Timeline|Scale Play)
        (:Update
          (Utilities|FlowControl|Sequence
            (:then_0
              (CallFunction|SetColor _accel))
            (:then_1
              (CallFunction|ChangeMaterials _accel))
            (:then_2
              (CallFunction|ScaleObjects _scale))))))))

(event EventTick
  (params (DeltaSeconds :type Float%20%28single-precision%29))
  (bind _accel (Timeline|Acceleration Play)
    (:Update
      (bind _scale (Timeline|Scale Play)
        (:Update
          (Utilities|FlowControl|Sequence
            (:then_0
              (CallFunction|SetColor _accel))
            (:then_1
              (CallFunction|ChangeMaterials _accel))
            (:then_2
              (CallFunction|ScaleObjects _scale))))))))

(fn ConstructionScript
  (bind _plane (Variables|Default|GetPlane))
  (bind _plane_2 (Variables|Default|GetPlane))
  (bind _plane_3 (Variables|Default|GetPlane))
  (Utilities|FlowControl|Sequence
    (:then_0
      (Variables|Default|SetoriginScale (Variables|/Script/Engine.SceneComponent|GetRelativeScale3D (Variables|Default|GetDefaultSceneRoot)))
      (Rendering|Material|CreateDynamicMaterialInstance (Variables|Default|GetPlane) 0 "/Game/VaporwaveAssets/Materials/M_Accel.M_Accel" "None" :!class /Script/Engine.PrimitiveComponent)
      ;[1 1 1] UV Scaling
      (Rendering|Material|SetScalarParameterValueonMaterials _plane "UScale" (Variables|Default|GetUScale))
      (Rendering|Material|SetScalarParameterValueonMaterials _plane "VScale" (Variables|Default|GetVScale))
      ;[1 1 1] Arrows Speed
      (Rendering|Material|SetScalarParameterValueonMaterials _plane_2 "arrowSpeed" (Variables|Default|GetArrowSpeed))
      (Rendering|Material|SetScalarParameterValueonMaterials _plane_2 "parallaxSpeed" (Variables|Default|GetParallaxSpeed))
      ;[1 1 1] Colors
      (Rendering|Material|SetVectorParameterValueonMaterials _plane_3 "AccelColor" (Math|Conversions|ToVector(LinearColor) (Variables|Default|Getcol1)))
      (Rendering|Material|SetVectorParameterValueonMaterials _plane_3 "ReverseColor" (Math|Conversions|ToVector(LinearColor) (Variables|Default|Getcol2))))
    (:then_1
      (Variables|Default|SetaccelMiddle 0.5))))

(fn ScaleObjects
  (params (Alpha :type Float%20%28double-precision%29))
  (bind _originscale (Variables|Default|GetoriginScale))
  (Transformation|SetRelativeScale3D (Variables|Default|GetDefaultSceneRoot) (Math|Vector|MakeVector (* Alpha (.x _originscale)) (.y _originscale) (.z _originscale))))

(fn SetColor
  (params (Alpha :type Float%20%28double-precision%29))
  (Rendering|Material|SetVectorParameterValueonMaterials (Variables|Default|GetPlane) "Color" (Math|Conversions|ToVector(LinearColor) (Math|Color|Lerp(LinearColor) (Variables|Default|Getcol1) (Variables|Default|Getcol2) Alpha))))

(fn ChangeMaterials
  (params (AccelAlpha :type Float%20%28double-precision%29))
  (Rendering|Material|SetScalarParameterValueonMaterials (Variables|Default|GetPlane) "AccelValue" AccelAlpha))

(fn AccelPlayer
  (params (IsAccelerate :type Boolean) (PlayerObject :type Actor%20Object%20Reference))
  (bind _asbp_third_person_character (Utilities|Casting|CastToBP_ThirdPersonCharacter PlayerObject))
  (Character|LaunchCharacter _asbp_third_person_character (Math|Vector|SelectVector (Math|Vector|MakeVector (Variables|Default|GetxAcceleration) 0.0 0.0) (Math|Vector|MakeVector (* (Variables|Default|GetxAcceleration) -1.0) 0.0 0.0) IsAccelerate) false false))