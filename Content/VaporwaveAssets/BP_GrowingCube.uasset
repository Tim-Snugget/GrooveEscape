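; Vaporwave cube actor that grows vertically and glows in step with a timeline.
; TimelineBump, started on BeginPlay and re-played every Tick, lerps the root's Z scale between min and max sizes.
; The same curve drives the "Main Power" material parameter on meshes tagged VaporEdge.
; When the third-person character leaves the Box, a Mario falling sound plays at the player's location.
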(event OnComponentEndOverlap(Box)
  (params (OverlappedComponent :type Primitive%20Component%20Object%20Reference) (OtherActor :type Actor%20Object%20Reference) (OtherComp :type Primitive%20Component%20Object%20Reference) (OtherBodyIndex :type Integer))
  (Utilities|Casting|CastToBP_ThirdPersonCharacter OtherActor)
  (Audio|PlaySoundatLocation "/Game/VaporwaveAssets/Sounds/Mario-Fall-Waa-Sound-Effect.Mario-Fall-Waa-Sound-Effect" (Transformation|GetWorldLocation (Variables|/Script/Engine.Actor|GetRootComponent (Game|GetPlayerCharacter 0))) "0, 0, 0" 1.0 1.0 0.0 0 0 0 0))

(event EventBeginPlay
  (bind _defaultsceneroot (Variables|Default|GetDefaultSceneRoot))
  (bind _relativescale3d (Variables|/Script/Engine.SceneComponent|GetRelativeScale3D _defaultsceneroot))
  (bind _bumperscaler (Timeline|timelineBump Play)
    (:Update
      ;[1 1 1] Scale VaporCube
      (Transformation|SetRelativeScale3D _defaultsceneroot (Math|Vector|MakeVector (.x _relativescale3d) (.y _relativescale3d) (Math|Float|Lerp (Variables|Default|GetminSizeScale) (Variables|Default|GetmaxSizeScale) _bumperscaler)))
      ;[1 1 1] Make the VaporCube's edges go WOOOOSH
      (for _array_element (Actor|GetComponentsbyTag "/Script/Engine.StaticMeshComponent" "VaporEdge")
        (Rendering|Material|SetScalarParameterValueonMaterials _array_element "Main Power" (Math|Float|Lerp 1.0 1423.0 _bumperscaler))))))

(event Collision|EventActorBeginOverlap
  (params (OtherActor :type Actor%20Object%20Reference)))

(event EventTick
  (params (DeltaSeconds :type Float%20%28single-precision%29))
  (bind _defaultsceneroot (Variables|Default|GetDefaultSceneRoot))
  (bind _relativescale3d (Variables|/Script/Engine.SceneComponent|GetRelativeScale3D _defaultsceneroot))
  (bind _bumperscaler (Timeline|timelineBump Play)
    (:Update
      ;[1 1 1] Scale VaporCube
      (Transformation|SetRelativeScale3D _defaultsceneroot (Math|Vector|MakeVector (.x _relativescale3d) (.y _relativescale3d) (Math|Float|Lerp (Variables|Default|GetminSizeScale) (Variables|Default|GetmaxSizeScale) _bumperscaler)))
      ;[1 1 1] Make the VaporCube's edges go WOOOOSH
      (for _array_element (Actor|GetComponentsbyTag "/Script/Engine.StaticMeshComponent" "VaporEdge")
        (Rendering|Material|SetScalarParameterValueonMaterials _array_element "Main Power" (Math|Float|Lerp 1.0 1423.0 _bumperscaler))))))

(fn ConstructionScript)