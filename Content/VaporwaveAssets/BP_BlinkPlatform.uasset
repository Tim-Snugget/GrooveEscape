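; Platform that blinks in and out of existence at a rhythm set by its BPM.
; BeginPlay starts a looping timer with an interval of one beat and a configurable start delay, calling Wall to toggle the mesh's visibility and collision together.
; The construction script applies the Color variable to the platform's materials.
; An older timeline-driven fade through the material's Appearance parameter remains in the graph but never runs.
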(event Custom|Wall
  (bind _plateform (Variables|Default|Getplateform))
  ;[1 1 1] Enable or Disable visuals/collisions depending of the current state of the object
  (if (Rendering|IsVisible _plateform)
    (Rendering|SetVisibility _plateform false false)
    (Collision|SetCollisionEnabled _plateform "NoCollision")
    (else
      (Rendering|SetVisibility _plateform true false)
      (Collision|SetCollisionEnabled _plateform "QueryAndPhysics"))))

(event EventBeginPlay
  ;[1 1 1] 1 - Setting the timer
  (Utilities|Time|SetTimerbyFunctionName 0 "Wall" (/ 6e+01 (Variables|Default|GetBPM)) true (Variables|Default|GetDelayAnimS)))

(fn ConstructionScript
  (Rendering|Material|SetVectorParameterValueonMaterials (Variables|Default|Getplateform) "Color" (Math|Conversions|ToVector(LinearColor) (Variables|Default|GetColor))))