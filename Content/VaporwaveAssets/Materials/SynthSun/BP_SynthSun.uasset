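; BP_SynthSun is a synthwave sun actor that pairs a glowing sphere with a spot light.
; The construction script configures the light and creates an M_SynthSun dynamic material instance for glow, animation speed and colors, though both color parameter names are None.
; With UseTwoColors on, BeginPlay or an actor overlap plays the SunLight timeline, which blends the light color from ColorOne to ColorTwo.
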(event EventBeginPlay
  (if (Variables|Default|GetUseTwoColors)
    (bind _lighting (Timeline|Sun%20Light Play)
      (:Update
        (Rendering|Components|Light|SetLightColor (Variables|Default|GetSpotLight) (Math|Color|Lerp(LinearColor) (Variables|Default|GetColorOne) (Variables|Default|GetColorTwo) _lighting) true)))))

(event Collision|EventActorBeginOverlap
  (params (OtherActor :type Actor%20Object%20Reference))
  (if (Variables|Default|GetUseTwoColors)
    (bind _lighting (Timeline|Sun%20Light Play)
      (:Update
        (Rendering|Components|Light|SetLightColor (Variables|Default|GetSpotLight) (Math|Color|Lerp(LinearColor) (Variables|Default|GetColorOne) (Variables|Default|GetColorTwo) _lighting) true)))))

(event EventTick
  (params (DeltaSeconds :type Float%20%28single-precision%29)))

(fn ConstructionScript
  (bind _spotlight (Variables|Default|GetSpotLight))
  (bind _colorone (Variables|Default|GetColorOne))
  (Utilities|FlowControl|Sequence
    (:then_0
      (Rendering|Components|Light|SetCastShadows _spotlight (Variables|Default|GetCastShadows))
      (Class|LightComponent|SetUseTemperature _spotlight (Variables|Default|GetUseTemperature))
      (Rendering|Components|Light|SetIntensity _spotlight (* (Variables|Default|GetIntensity) 1e+04)))
    (:then_1
      (bind _returnvalue (Rendering|Material|CreateDynamicMaterialInstance (Variables|Default|GetSphere) 0 "/Game/VaporwaveAssets/Materials/SynthSun/M_SynthSun.M_SynthSun" "None" :!class /Script/Engine.PrimitiveComponent))
      (Rendering|Material|SetScalarParameterValue _returnvalue "EmissivePower" (Variables|Default|GetEmissivePower) :!class /Script/Engine.MaterialInstanceDynamic)
      (Rendering|Material|SetScalarParameterValue _returnvalue "AnimSpeed" (Variables|Default|GetAnimSpeed) :!class /Script/Engine.MaterialInstanceDynamic)
      (Rendering|Material|SetVectorParameterValue _returnvalue "None" _colorone :!class /Script/Engine.MaterialInstanceDynamic)
      (Rendering|Material|SetVectorParameterValue _returnvalue "None" (Math|Color|SelectColor (Variables|Default|GetColorTwo) _colorone (Variables|Default|GetUseTwoColors)) :!class /Script/Engine.MaterialInstanceDynamic))))