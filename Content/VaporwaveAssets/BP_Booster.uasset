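; Booster pad that launches the third-person character forward or backward along its X axis when they enter its box.
; Ground friction and walking braking are saved and zeroed on entry, then restored on exit.
; If bidirectional, an Acceleration timeline sets launch direction and drives arrow material color and value; otherwise it always accelerates.
; A nested Scale timeline stretches the pad along X, and construction configures the dynamic material.
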(event OnComponentBeginOverlap(Box)
  (params (OverlappedComponent :type Primitive%20Component%20Object%20Reference) (OtherActor :type Actor%20Object%20Reference) (OtherComp :type Primitive%20Component%20Object%20Reference) (OtherBodyIndex :type Integer) (bFromSweep :type Boolean) (SweepResult :type Hit%20Result%20Structure%20%28by%20ref%29))
  (bind _asbp_third_person_character (Utilities|Casting|CastToBP_ThirdPersonCharacter OtherActor))
  (CallFunction|AccelPlayer (> (Math|Float|SelectFloat (stale EventBeginPlay _accel) 1.0 (Variables|Default|GetisBidirectionalBooster)) 0.5) _asbp_third_person_character))

(event OnComponentEndOverlap(Box)
  (params (OverlappedComponent :type Primitive%20Component%20Object%20Reference) (OtherActor :type Actor%20Object%20Reference) (OtherComp :type Primitive%20Component%20Object%20Reference) (OtherBodyIndex :type Integer))
  (bind _asbp_third_person_character (Utilities|Casting|CastToBP_ThirdPersonCharacter OtherActor))
  ;[1 1 1] out of the booster, player's friction & braking is reset
  (Variables|/Script/Engine.CharacterMovementComponent|SetGroundFriction (Variables|/Script/Engine.Character|GetCharacterMovement _asbp_third_person_character) (Variables|Default|GetgroundFrictionPlayer))
  (Variables|/Script/Engine.CharacterMovementComponent|SetBrakingDecelerationWalking (Variables|/Script/Engine.Character|GetCharacterMovement _asbp_third_person_character) (Variables|Default|GetbrakingDWPlayer)))

(event EventBeginPlay
  (bind _accel (Timeline|Acceleration Play)
    (:Update
      (bind _scale (Timeline|Scale Play)
        (:Update
          (Utilities|FlowControl|Sequence
            (:then_0
              (CallFunction|SetColor (Math|Float|SelectFloat _accel 1.0 (Variables|Default|GetisBidirectionalBooster))))
            (:then_1
              (CallFunction|ChangeMaterials (Math|Float|SelectFloat _accel 1.0 (Variables|Default|GetisBidirectionalBooster))))
            (:then_2
              (CallFunction|ScaleObjects _scale))))))))

(event EventTick
  (params (DeltaSeconds :type Float%20%28single-precision%29))
  (bind _accel (Timeline|Acceleration Play)
    (:Update
      (bind _scale (Timeline|Scale Play)
        (:Update
          (Utilities|FlowControl|Sequence
            (:then_0
              (CallFunction|SetColor (Math|Float|SelectFloat _accel 1.0 (Variables|Default|GetisBidirectionalBooster))))
            (:then_1
              (CallFunction|ChangeMaterials (Math|Float|SelectFloat _accel 1.0 (Variables|Default|GetisBidirectionalBooster))))
            (:then_2
              (CallFunction|ScaleObjects _scale))))))))

(fn ConstructionScript
  (bind _plane (Variables|Default|GetPlane))
  (bind _plane_2 (Variables|Default|GetPlane))
  (bind _plane_3 (Variables|Default|GetPlane))
  (Variables|Default|SetoriginScale (Variables|/Script/Engine.SceneComponent|GetRelativeScale3D (Variables|Default|GetDefaultSceneRoot)))
  (Rendering|Material|CreateDynamicMaterialInstance (Variables|Default|GetPlane) 0 "/Game/VaporwaveAssets/Materials/Booster/M_Accel.M_Accel" "None" :!class /Script/Engine.PrimitiveComponent)
  ;[1 1 1] UV Scaling
  (Rendering|Material|SetScalarParameterValueonMaterials _plane "UScale" (Variables|Default|GetUScale))
  (Rendering|Material|SetScalarParameterValueonMaterials _plane "VScale" (Variables|Default|GetVScale))
  ;[1 1 1] Arrows Speed
  (Rendering|Material|SetScalarParameterValueonMaterials _plane_2 "arrowSpeed" (Variables|Default|GetArrowSpeed))
  (Rendering|Material|SetScalarParameterValueonMaterials _plane_2 "parallaxSpeed" (Variables|Default|GetParallaxSpeed))
  ;[1 1 1] Colors
  (Rendering|Material|SetVectorParameterValueonMaterials _plane_3 "AccelColor" (Math|Conversions|ToVector(LinearColor) (Variables|Default|Getcol1)))
  (Rendering|Material|SetVectorParameterValueonMaterials _plane_3 "ReverseColor" (Math|Conversions|ToVector(LinearColor) (Variables|Default|Getcol2))))

(fn ScaleObjects
  (params (Alpha :type Float%20%28double-precision%29))
  (bind _originscale (Variables|Default|GetoriginScale))
  (Transformation|SetRelativeScale3D (Variables|Default|GetDefaultSceneRoot) (Math|Vector|MakeVector (* Alpha (.x _originscale)) (.y _originscale) (.z _originscale))))

(fn SetColor
  (params (Alpha :type Float%20%28double-precision%29))
  (Rendering|Material|SetVectorParameterValueonMaterials (Variables|Default|GetPlane) "Color" (Math|Conversions|ToVector(LinearColor) (Math|Color|Lerp(LinearColor) (Variables|Default|Getcol1) (Variables|Default|Getcol2) Alpha))))

(fn ChangeMaterials
  (params (AccelAlpha :type Float%20%28double-precision%29))
  (Rendering|Material|SetScalarParameterValueonMaterials (Variables|Default|GetPlane) "AccelValue" AccelAlpha))

(fn AccelPlayer
  (params (IsAccelerate :type Boolean) (PlayerObject :type Actor%20Object%20Reference))
  (bind _accelvalue (Variables|Default|GetaccelValue))
  (bind _asbp_third_person_character (Utilities|Casting|CastToBP_ThirdPersonCharacter PlayerObject))
  (Utilities|FlowControl|Sequence
    (:then_0
      ;[1 1 1] Save default friction and braking values
      (Variables|Default|SetgroundFrictionPlayer (Variables|/Script/Engine.CharacterMovementComponent|GetGroundFriction (Variables|/Script/Engine.Character|GetCharacterMovement _asbp_third_person_character)))
      (Variables|Default|SetbrakingDWPlayer (Variables|/Script/Engine.CharacterMovementComponent|GetBrakingDecelerationWalking (Variables|/Script/Engine.Character|GetCharacterMovement _asbp_third_person_character))))
    (:then_1
      ;[1 1 1] Disabling friction and values
      (Variables|/Script/Engine.CharacterMovementComponent|SetGroundFriction (Variables|/Script/Engine.Character|GetCharacterMovement _asbp_third_person_character) 0.0)
      (Variables|/Script/Engine.CharacterMovementComponent|SetBrakingDecelerationWalking (Variables|/Script/Engine.Character|GetCharacterMovement _asbp_third_person_character) 0.0))
    (:then_3
      ;[1 1 1] Apply force to the player depending on the booster's rotation
      (Character|LaunchCharacter _asbp_third_person_character (* (Math|Rotator|GetRotationXVector (Transformation|GetWorldRotation (Variables|Default|GetDefaultSceneRoot))) (Math|Float|SelectFloat _accelvalue (* _accelvalue -1.0) IsAccelerate)) false false))))