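; Checkpoint actor that sets the player's respawn point and marks its location with a configurable spotlight.
; On box overlap by BP_ThirdPersonCharacter, it stores the box transform as that character's RespawnTransform, then plays a sound and a short-lived particle burst.
; The construction script applies light color and intensity and caches the outer cone angle.
; A timeline, played from BeginPlay and Tick, animates that angle from a multiplied width toward the cached one.
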(event OnComponentBeginOverlap(Box)
  (params (OverlappedComponent :type Primitive%20Component%20Object%20Reference) (OtherActor :type Actor%20Object%20Reference) (OtherComp :type Primitive%20Component%20Object%20Reference) (OtherBodyIndex :type Integer) (bFromSweep :type Boolean) (SweepResult :type Hit%20Result%20Structure%20%28by%20ref%29))
  (bind _defaultsceneroot (Variables|Default|GetDefaultSceneRoot))
  (bind _returnvalue (Transformation|GetWorldLocation _defaultsceneroot))
  (bind _asbp_third_person_character (Utilities|Casting|CastToBP_ThirdPersonCharacter OtherActor))
  (Utilities|FlowControl|Sequence
    (:then_0
      ;[1 1 1] Set new respawn location
      (Variables|/Game/ThirdPerson/Blueprints/BP_ThirdPersonCharacter.BP_ThirdPersonCharacter_C|SetRespawnTransform _asbp_third_person_character (Transformation|GetWorldTransform (Variables|Default|GetBox))))
    (:then_1
      (Audio|PlaySoundatLocation "/Engine/EditorSounds/Notifications/CompileSuccess.CompileSuccess" _returnvalue "0, 0, 0" 1.0 1.0 0.0 0 0 0 0)
      (bind _returnvalue_2 (Effects|SpawnEmitteratLocation "/Game/FXVarietyPack/Particles/P_ky_thunderBall.P_ky_thunderBall" _returnvalue))
      (Utilities|FlowControl|Delay 0.75)
      (Components|DestroyComponent _returnvalue_2))))

(event EventBeginPlay
  (bind _outercone (Variables|Default|GetouterCone))
  (bind _lightwidth (Timeline|lightWidth Play)
    (:Update
      (Rendering|Lighting|SetOuterConeAngle (Variables|Default|GetSpotLight) (Math|Float|Lerp (* _outercone (Variables|Default|GetOuterConeMultiplier)) _outercone _lightwidth)))))

(event Collision|EventActorBeginOverlap
  (params (OtherActor :type Actor%20Object%20Reference)))

(event EventTick
  (params (DeltaSeconds :type Float%20%28single-precision%29))
  (bind _outercone (Variables|Default|GetouterCone))
  (bind _lightwidth (Timeline|lightWidth Play)
    (:Update
      (Rendering|Lighting|SetOuterConeAngle (Variables|Default|GetSpotLight) (Math|Float|Lerp (* _outercone (Variables|Default|GetOuterConeMultiplier)) _outercone _lightwidth)))))

(fn ConstructionScript
  (bind _spotlight (Variables|Default|GetSpotLight))
  (Rendering|Components|Light|SetIntensity _spotlight (* (Variables|Default|GetLight%20Intensity) 5e+03))
  (Rendering|Components|Light|SetLightColor _spotlight (Variables|Default|GetLight%20Color) true)
  (Variables|Default|SetouterCone (Variables|/Script/Engine.SpotLightComponent|GetOuterConeAngle _spotlight)))